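; BP_Nuage is a cloud platform that briefly disappears after the player character touches it.
; When the BP_CharacterPawn instance overlaps its Box trigger, a one-second delay runs, then the Cube is hidden and both components ignore collision.
; After another second, the Box overlaps pawns again and the Cube becomes visible and blocking, so the cycle can repeat.
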(event OnComponentBeginOverlap(Box)
  (params (OverlappedComponent :type Primitive%20Component%20Object%20Reference) (OtherActor :type Actor%20Object%20Reference) (OtherComp :type Primitive%20Component%20Object%20Reference) (OtherBodyIndex :type Integer) (bFromSweep :type Boolean) (SweepResult :type Hit%20Result%20Structure%20%28by%20ref%29))
  (bind _returnvalue (Actor|GetActorOfClass "/Game/Blueprint/Player/BP_CharacterPawn.BP_CharacterPawn_C"))
  (if (== OtherActor _returnvalue)
    (Utilities|FlowControl|Delay 1.0)
    (Collision|SetCollisionResponsetoAllChannels (Variables|Default|GetCube) "ECR_Ignore")
    (Collision|SetCollisionResponsetoChannel (Variables|Default|GetCube) "ECC_Pawn" "ECR_Ignore")
    (Rendering|SetVisibility (Variables|Default|GetCube) false false)
    (Utilities|FlowControl|Delay 1.0)
    (Collision|SetCollisionResponsetoChannel (Variables|Default|GetBox) "ECC_Pawn" "ECR_Overlap")
    (Collision|SetCollisionResponsetoAllChannels (Variables|Default|GetCube) "ECR_Block")
    (Rendering|SetVisibility (Variables|Default|GetCube) true false)))

(fn ConstructionScript)