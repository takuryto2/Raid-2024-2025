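; BP_Checkpoint is a checkpoint actor that records the current fog height when a player-controlled actor overlaps it.
; On overlap it checks the actor's Instigator, copies FogHeight from the BP_FogTest found in the level into SavedFogHeight, and turns its Cube green.
; The Used flag starts true at BeginPlay and is never cleared, so every qualifying overlap saves again.
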(event Collision|EventActorBeginOverlap
  (params (OtherActor :type Actor%20Object%20Reference))
  (if (Variables|Default|GetUsed)
    (if (Pawn|IsPlayerControlled (Variables|/Script/Engine.Actor|GetInstigator OtherActor))
      (Variables|Default|SetUsed true)
      ;[0.15 0.15 0.15 0.5] Save Fog Height
      (bind _returnvalue (Actor|GetActorOfClass "/Game/Checkpoint/BP_FogTest.BP_FogTest_C"))
      (Variables|Default|SetSavedFogHeight (Variables|/Game/Checkpoint/BP_FogTest.BP_FogTest_C|GetFog%20Height _returnvalue))
      ;[0.15 0.15 0.15 0.5] Visual
      (Rendering|Material|SetMaterial (Variables|Default|GetCube) 0 "/AnimationSharing/AnimSharingGreen.AnimSharingGreen"))))

(event EventBeginPlay
  (Variables|Default|SetUsed true))

(fn ConstructionScript)