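; BP_CharacterPawn is a player pawn that serves as the view target and keeps its pivot turning with the tower.
; On BeginPlay it sets the player's view to itself and hands PivotBP to BP_Tower as its PlayerCameraPivot.
; Each Tick it looks up BP_Tower again and copies the TowerPivot world rotation onto PivotBP.
; The R key toggles pause through BP_GameInstance, and ShouldRecreate always returns true.
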(event EventBeginPlay
  (Game|Player|SetViewTargetwithBlend (Game|GetPlayerController (Variables|/Script/Engine.Pawn|GetPlayerState (Game|Player|GetPlayerPawn 0))) self 0.0 "VTBlend_Linear" 0.0 false)
  (bind _returnvalue (Actor|GetActorOfClass "/Game/Blueprint/Tower/BP_Tower.BP_Tower_C"))
  (Variables|/Script/Raid_2024_2025.Tower|SetplayerCameraPivot _returnvalue (Variables|Default|GetPivot%20BP)))

(event EventTick
  (params (DeltaSeconds :type Float%20%28single-precision%29))
  (bind _returnvalue (Actor|GetActorOfClass "/Game/Blueprint/Tower/BP_Tower.BP_Tower_C"))
  (Transformation|SetWorldRotation (Variables|Default|GetPivot%20BP) (Transformation|GetWorldRotation (Variables|/Game/Blueprint/Tower/BP_Tower.BP_Tower_C|GetTowerPivot _returnvalue)) false false))

(event Input|KeyboardEvents|R
  (params (Key :type Key%20Structure :default "None"))
  (:Pressed
    (bind _asbp_game_instance (Utilities|Casting|CastToBP_GameInstance (Game|GetGameInstance)))
    (Default|TogglePause _asbp_game_instance)))

(fn ConstructionScript)

(fn ShouldRecreate
  (return true))