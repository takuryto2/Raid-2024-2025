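; MovingLaser is a level design actor that slides its static mesh back and forth between two relative positions.
; On BeginPlay, two custom events, MoveRight and MoveLeft, call each other after each three-second latent MoveComponentTo, forming an endless ping-pong toward Pos1 and Pos2.
; The graph contains only movement, with no collision or damage logic.
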(event Custom|MoveRight
  (Components|MoveComponentTo (Variables|Default|GetStaticMesh) (Variables|Default|GetPos1) "0, 0, 0" false false 3.0 false)
  (CallFunction|MoveLeft))

(event Custom|MoveLeft
  (Components|MoveComponentTo (Variables|Default|GetStaticMesh) (Variables|Default|GetPos2) "0, 0, 0" false false 3.0 false)
  (CallFunction|MoveRight))

(event EventBeginPlay
  (CallFunction|MoveRight))

(fn ConstructionScript)