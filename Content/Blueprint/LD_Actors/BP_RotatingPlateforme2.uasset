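; BP_RotatingPlateforme2 is a level-design platform that orbits a center in a vertical circle around the world Y axis, without changing its own orientation.
; Tick accumulates an angle from speed and direction, then RotateActorAroundPoint rotates a radius offset by that plus a starting angle.
; The center follows TargetActor when valid, otherwise the spawn location.
; Movement is unswept; the RotateVectorAroundPoint helper is unused.
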(event EventTick
  (params (DeltaSeconds :type Float%20%28single-precision%29))
  (Variables|Default|SetCurrent%20Rotation (+ (Variables|Default|GetCurrent%20Rotation) (* (* (Variables|Default|GetRotation%20Speed) DeltaSeconds) (Math|Float|SelectFloat 1.0 -1.0 (Variables|Default|GetClockwise)))))
  (CallFunction|RotateActorAroundPoint self (Variables|Default|GetTarget%20Actor) (Variables|Default|GetInitial%20Location) (Variables|Default|GetRadius) (Variables|Default|GetStarting%20Angle) (Variables|Default|GetCurrent%20Rotation)))

(event EventBeginPlay
  (Variables|Default|SetInitial%20Location (Transformation|GetActorLocation)))

(fn ConstructionScript)

(fn RotateVectorAroundPoint
  (params (Pivot%20Vector :type Vector) (Vector%20to%20Rotate :type Vector) (Rotation :type Rotator))
  (bind _returnvalue (Math|Conversions|ToTransform(Vector) Pivot%20Vector))
  (return (Math|Transform|TransformLocation _returnvalue (Math|Vector|RotateVector (Math|Transform|InverseTransformLocation _returnvalue Vector%20to%20Rotate) Rotation))))

(fn RotateActorAroundPoint
  (params (ActorToRotate :type Actor%20Object%20Reference) (TargetActor :type Actor%20Object%20Reference) (TargetLocation :type Vector) (Radius :type Float%20%28double-precision%29) (Angle :type Float%20%28double-precision%29) (RotationPoint :type Float%20%28double-precision%29))
  (LocalVariables|SetLActorToRotate ActorToRotate)
  (LocalVariables|SetLTargetActor TargetActor)
  (LocalVariables|SetLLocation TargetLocation)
  (LocalVariables|SetLoRadius Radius)
  (LocalVariables|SetLAngle Angle)
  (LocalVariables|SetLRate RotationPoint)
  (Utilities|IsValid (LocalVariables|GetLTargetActor)
    (:Is%20Valid
      (LocalVariables|SetLLocation (Transformation|GetActorLocation (LocalVariables|GetLTargetActor))))
    (:Is%20Not%20Valid
      _))
  (Transformation|SetActorLocation (LocalVariables|GetLActorToRotate) (+ (LocalVariables|GetLLocation) (Math|Vector|RotateVectorAroundAxis (Math|Vector|MakeVectorNetQuantize 0.0 0.0 (LocalVariables|GetLoRadius)) (+ (LocalVariables|GetLRate) (LocalVariables|GetLAngle)) "0.000000,1.000000,0.000000")) false false)
  (return (LocalVariables|GetLLocation)))