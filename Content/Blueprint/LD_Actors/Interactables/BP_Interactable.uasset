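; Base interactable actor that lets the player toggle it on and off with the F key while inside its collision box.
; Box overlaps with the player pawn set whether interaction is allowed; the box can be disabled at start through a flag.
; Each interaction flips the activated state, plays an activate or deactivate sound, then calls Interact, a placeholder that only prints.
; GetState and ShouldRecreate are stubs, apparently meant for child overrides.
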(event OnComponentBeginOverlap(Box)
  (params (OverlappedComponent :type Primitive%20Component%20Object%20Reference) (OtherActor :type Actor%20Object%20Reference) (OtherComp :type Primitive%20Component%20Object%20Reference) (OtherBodyIndex :type Integer) (bFromSweep :type Boolean) (SweepResult :type Hit%20Result%20Structure%20%28by%20ref%29))
  (if (== OtherActor (Variables|Default|Getcharacter))
    (Variables|Default|SetcanInteract true)
    (CallFunction|OnCanInteract)))

(event OnComponentEndOverlap(Box)
  (params (OverlappedComponent :type Primitive%20Component%20Object%20Reference) (OtherActor :type Actor%20Object%20Reference) (OtherComp :type Primitive%20Component%20Object%20Reference) (OtherBodyIndex :type Integer))
  (if (== (Variables|Default|Getcharacter) OtherActor)
    (Variables|Default|SetcanInteract false)
    (CallFunction|OnCantInteract)))

(event EventBeginPlay
  (bind _asbp_character_pawn (Utilities|Casting|CastToBP_CharacterPawn (Game|Player|GetPlayerPawn 0)))
  (Variables|Default|Setcharacter _asbp_character_pawn)
  (if (not (Variables|Default|GetuseCollisionBox))
    (CallFunction|DisableCollisionBox)))

(event Input|KeyboardEvents|F
  (params (Key :type Key%20Structure :default "None"))
  (:Pressed
    (Development|PrintString (Variables|Default|Getname))
    (if (Variables|Default|GetcanInteract)
      (CallFunction|CallInteract))))

(fn ConstructionScript)

(fn DisableCollisionBox
  (Collision|SetCollisionEnabled (Variables|Default|GetBox) "NoCollision"))

(fn EnableCollisionBox
  (Collision|SetCollisionEnabled (Variables|Default|GetBox) "QueryOnly"))

(fn OnCanInteract
  (Development|PrintText (Utilities|Text|FormatText "Can interact with {name}" (Variables|Default|Getname))))

(fn OnCantInteract
  (Development|PrintText (Utilities|Text|FormatText "Can't interact with {name}" (Variables|Default|Getname))))

(fn CallInteract
  (bind _output_get (Variables|Default|Setactivated (not (Variables|Default|Getactivated))))
  (if _output_get
    (CallFunction|PlayifValid (Variables|Default|GetactivateSound))
    (else
      (CallFunction|PlayifValid (Variables|Default|GetdeactivateSound))))
  (CallFunction|Interact _output_get))

(fn Interact
  (params (Activate :type Boolean))
  (Development|PrintText (Utilities|Text|FormatText "Interact not implemented for {name}" (Variables|Default|Getname))))

(fn GetState
  (return ""))

(fn ShouldRecreate
  (return true))