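; BP_Rail is a level-design actor that builds a rail mesh along an editable spline.
; Its construction script adds a spline mesh component between each pair of neighboring points, matching their local positions and tangents and using MainSplineMesh along the X axis.
; ValidateMeshes defaults an unset intermediate mesh to the main one and overwrites first and last meshes when they are set, though segment building uses none of these.
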(event EventBeginPlay)

(fn ConstructionScript
  (bind _spline (Variables|Default|GetSpline))
  (bind _spline_2 (Variables|Default|GetSpline))
  (bind _spline_3 (Variables|Default|GetSpline))
  (bind _returnvalue (Spline|GetNumberOfSplinePoints _spline))
  (Variables|Default|GetMainSplineMesh
    (:then
      (CallFunction|ValidateMeshes)
      (LocalVariables|SetNumberOfSplinePoints _returnvalue)
      (for _index (range 0 (- _returnvalue 1))
        (LocalVariables|SetCurrentIndex _index)
        (if (< (+ _index 1) (LocalVariables|GetNumberOfSplinePoints))
          (bind _returnvalue_2 (AddComponent|AddSplineMeshComponent false))
          (SplineMesh|SetStartandEnd _returnvalue_2 (.location (Spline|GetTransformatSplinePoint _spline_2 (LocalVariables|GetCurrentIndex) "Local" false)) (Spline|GetTangentatSplinePoint _spline_3 (LocalVariables|GetCurrentIndex) "Local") (.location (Spline|GetTransformatSplinePoint _spline_2 (+ _index 1) "Local" false)) (Spline|GetTangentatSplinePoint _spline_3 (+ (LocalVariables|GetCurrentIndex) 1) "Local") true :!class /Script/Engine.SplineMeshComponent)
          (Components|StaticMesh|SetStaticMesh _returnvalue_2 (Variables|Default|GetMainSplineMesh))
          (SplineMesh|SetForwardAxis _returnvalue_2 "X" true))))
    (:else)))

(fn ValidateMeshes
  (bind _mainsplinemesh (Variables|Default|GetMainSplineMesh))
  (Utilities|FlowControl|Sequence
    (:then_0
      (Variables|Default|GetIntermediateSplineMesh
        (:then)
        (:else
          (Variables|Default|SetIntermediateSplineMesh _mainsplinemesh))))
    (:then_1
      (Variables|Default|GetFirstMesh
        (:then
          (Variables|Default|SetFirstMesh _mainsplinemesh))
        (:else)))
    (:then_2
      (Variables|Default|GetLastMesh
        (:then
          (Variables|Default|SetLastMesh _mainsplinemesh))
        (:else)))))