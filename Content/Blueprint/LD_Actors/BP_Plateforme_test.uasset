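; BP_Plateforme_test is a test platform actor whose static mesh shuttles back and forth along its local X axis.
; From BeginPlay, two events call each other after each timed MoveComponentTo, looping between an offset and the relative origin.
; Every Tick, a valid MovableActor is snapped to the mesh's world location without sweep, so it follows the platform.
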(event Custom|PlateformeMoveRight
  (Components|MoveComponentTo (Variables|Default|GetStaticMesh) "800.000000,0.000000,0.000000" "0, 0, 0" false false 3.0 false)
  (CallFunction|PlateformeMoveLeft))

(event Custom|PlateformeMoveLeft
  (Components|MoveComponentTo (Variables|Default|GetStaticMesh) "0, 0, 0" "0, 0, 0" false false 3.0 false)
  (CallFunction|PlateformeMoveRight))

(event EventBeginPlay
  (CallFunction|PlateformeMoveRight))

(event EventTick
  (params (DeltaSeconds :type Float%20%28single-precision%29))
  (bind _movable_actor (Variables|Default|GetMovable%20actor))
  (Utilities|IsValid _movable_actor
    (:Is%20Valid
      (Transformation|SetActorLocation _movable_actor (Transformation|GetWorldLocation (Variables|Default|GetStaticMesh)) false false))))

(fn ConstructionScript)