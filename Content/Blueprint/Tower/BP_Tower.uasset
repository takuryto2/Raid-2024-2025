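; BP_Tower is a tower actor that takes over the player's camera view when play begins and can be told to rotate.
; On BeginPlay it copies its camera pivot and left and right anchors into working variables, stores the player pawn and blends the view target to itself.
; RotateTowerEvent forwards its parameter to TryTurn, whose logic is defined outside this graph.
; NewFunction is a debug stub that prints and returns its input.
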(event Custom|RotateTowerEvent
  (params (NewParam :type Float%20%28double-precision%29))
  (Class|Tower|TryTurn NewParam))

(event EventBeginPlay
  (bind _returnvalue (Game|Player|GetPlayerPawn 0))
  (Variables|Default|SetCameraPivot (Variables|Default|GetCamera%20Pivot%20BP))
  (Variables|Default|SetPlayerActor _returnvalue)
  (Game|Player|SetViewTargetwithBlend (Game|GetPlayerController (Variables|/Script/Engine.Pawn|GetPlayerState _returnvalue)) self 0.0 "VTBlend_Linear" 0.0 false)
  (Variables|Default|SetLeftAnchor (Variables|Default|GetbpLeftAnchor))
  (Variables|Default|SetRightAnchor (Variables|Default|GetbpRightAnchor)))

(fn ConstructionScript)

(fn NewFunction
  (params (NewParam :type Float%20%28double-precision%29))
  (Development|PrintString "AYO")
  (return NewParam))