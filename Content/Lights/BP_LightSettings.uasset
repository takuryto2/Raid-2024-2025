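; BP_LightSettings is a lighting settings actor that configures the level's sun, sky light, clouds and fog on BeginPlay.
; When InSceneLightActors is true it only hides its root and children; otherwise it runs one setup event per element.
; Each event finds its actor by class, then applies variable-driven light, cloud or fog properties.
; The directional and sky lights become Movable, and the directional light gets a fixed rotation.
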(event Custom|Set%20DirectionalLight
  ;[0.15 0.15 0.15 0.5] Directional Light
  (bind _returnvalue (Actor|GetActorOfClass "/Script/Engine.DirectionalLight"))
  (bind _output_get (Variables|Default|SetDirectionalLight _returnvalue))
  (Transformation|SetMobility (Variables|/Script/Engine.Light|GetLightComponent _output_get) "Movable")
  (Transformation|SetActorRotation _output_get "-3.000000,0.000000,0.000000")
  (Rendering|Components|Light|SetIntensity (Variables|/Script/Engine.Light|GetLightComponent _output_get) (Variables|Default|GetIntensity))
  (Rendering|Components|Light|SetLightColor (Variables|/Script/Engine.Light|GetLightComponent _output_get) (Variables|Default|GetLight%20Color) true)
  (Class|LightComponent|SetTemperature (Variables|/Script/Engine.Light|GetLightComponent _output_get) (Variables|Default|GetTemperature)))

(event Custom|SetSkyLight
  ;[0.15 0.15 0.15 0.5] Sky Light
  (bind _returnvalue (Actor|GetActorOfClass "/Script/Engine.SkyLight"))
  (bind _output_get (Variables|Default|SetSkylight _returnvalue))
  (Transformation|SetMobility (Variables|/Script/Engine.SkyLight|GetLightComponent _output_get) "Movable"))

(event Custom|SetVolumetricCloud
  ;[0.15 0.15 0.15 0.5] Volumetric Cloud
  (bind _returnvalue (Actor|GetActorOfClass "/Script/Engine.VolumetricCloud"))
  (Class|VolumetricCloudComponent|SetPlanetRadius (Variables|/Script/Engine.VolumetricCloud|GetVolumetricCloudComponent _returnvalue) (Variables|Default|GetPlanet%20Radius)))

(event Custom|SetHeightFog
  ;[0.15 0.15 0.15 0.5] Height Fog
  (bind _returnvalue (Actor|GetActorOfClass "/Script/Engine.ExponentialHeightFog"))
  (Class|ExponentialHeightFogComponent|SetFogDensity (Variables|/Script/Engine.ExponentialHeightFog|GetComponent _returnvalue) (Variables|Default|GetFog%20Density))
  (Class|ExponentialHeightFogComponent|SetSecondFogDensity (Variables|/Script/Engine.ExponentialHeightFog|GetComponent _returnvalue) (Variables|Default|GetSecond%20Fog%20Density))
  (Class|ExponentialHeightFogComponent|SetFogInscatteringColor (Variables|/Script/Engine.ExponentialHeightFog|GetComponent _returnvalue) (Variables|Default|GetFog%20Inscattering%20Color))
  (Class|ExponentialHeightFogComponent|SetVolumetricFog (Variables|/Script/Engine.ExponentialHeightFog|GetComponent _returnvalue) (Variables|Default|GetVolumetric%20Fog)))

(event EventBeginPlay
  (if (Variables|Default|GetInSceneLightActors)
    (Rendering|SetVisibility (Variables|Default|GetDefaultSceneRoot) false true)
    (else
      (CallFunction|SetDirectionalLight)
      (CallFunction|SetSkyLight)
      (CallFunction|SetVolumetricCloud)
      (CallFunction|SetHeightFog))))

(fn ConstructionScript)