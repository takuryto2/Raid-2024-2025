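; Game mode that provides save and load functions for game progress and settings, each with its own slot name and index.
; Save fills a new SaveGameObject from the game instance and writes it to its slot.
; Load and LoadSettings read their slot and pass the game instance to the saved object's Load.
; SaveSettings only creates and labels the object, as its slot write is disconnected.
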(event EventBeginPlay)

(event EventTick
  (params (DeltaSeconds :type Float%20%28single-precision%29)))

(fn ConstructionScript)

(fn Save
  (bind _saveslotname (Variables|Default|GetsaveSlotName))
  (bind _saveslotindex (Variables|Default|GetsaveSlotIndex))
  (bind _returnvalue (SaveGame|CreateSaveGameObject "/Script/Raid_2024_2025.SaveGameObject"))
  (Variables|/Script/Raid_2024_2025.SaveGameObject|SetslotName _returnvalue _saveslotname)
  (Variables|/Script/Raid_2024_2025.SaveGameObject|SetslotIndex _returnvalue _saveslotindex)
  (Class|SaveGameObject|Save _returnvalue (Game|GetGameInstance))
  (SaveGame|SaveGametoSlot _returnvalue _saveslotname _saveslotindex))

(fn Load
  (bind _returnvalue (SaveGame|LoadGamefromSlot (Variables|Default|GetsaveSlotName) (Variables|Default|GetsaveSlotIndex)))
  (bind _assave_game_object (Utilities|Casting|CastToSaveGameObject _returnvalue))
  (Class|SaveGameObject|Load _assave_game_object (Game|GetGameInstance)))

(fn SaveSettings
  (bind _returnvalue (SaveGame|CreateSaveGameObject "/Script/Raid_2024_2025.SaveGameObject"))
  (Variables|/Script/Raid_2024_2025.SaveGameObject|SetslotName _returnvalue (Variables|Default|GetsettingsSlotName))
  (Variables|/Script/Raid_2024_2025.SaveGameObject|SetslotIndex _returnvalue (Variables|Default|GetsettingsSlotIndex)))

(fn LoadSettings
  (bind _returnvalue (SaveGame|LoadGamefromSlot (Variables|Default|GetsettingsSlotName) (Variables|Default|GetsettingsSlotIndex)))
  (bind _assave_game_object (Utilities|Casting|CastToSaveGameObject _returnvalue))
  (Class|SaveGameObject|Load _assave_game_object (Game|GetGameInstance)))