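; Fog hazard actor that waits for a set delay, then grows upward over a fixed duration toward a maximum height.
; Tick runs FogMovement, which lerps the height and feeds it into the Niagara smoke's box size and spawn rate, so the volume grows without moving the actor.
; A debug-drawn box trace follows that height and only prints a placeholder string when it hits BP_CharacterPawn.
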(event EventBeginPlay
  (Actor|GetActorOfClass "/Game/FogBlueprints/bP_TestCube.bP_TestCube_C"))

(event EventTick
  (params (DeltaSeconds :type Float%20%28single-precision%29))
  (Variables|Default|SetdeltaSeconds DeltaSeconds)
  (Variables|Default|SetwaitTimer (+ (Variables|Default|GetwaitTimer) (Variables|Default|GetdeltaSeconds)))
  (if (>= (Variables|Default|GetwaitTimer) (Variables|Default|GetmaxWaitTimer))
    (CallFunction|FogMovement)))

(fn ConstructionScript)

(fn FogMovement
  (bind _maxmovetimer (Variables|Default|GetmaxMoveTimer))
  (bind _tracehalfsize (Variables|Default|GettraceHalfSize))
  (bind _output_get (Variables|Default|SetmoveTimer (+ (Variables|Default|GetmoveTimer) (Variables|Default|GetdeltaSeconds))))
  (Variables|Default|SetSpawnRatePaticles (/ (Variables|Default|GetCurrentHeight) 1.25))
  (Effects|Components|ParticleSystem|SetFloatParameter (Variables|Default|GetNS_StylizedSmoke) "SpawnRate" (Variables|Default|GetSpawnRatePaticles))
  (Variables|Default|SetisFogActive (>= _output_get _maxmovetimer))
  (if (not (>= _output_get _maxmovetimer))
    (Components|Activation|Activate (Variables|Default|GetNS_StylizedSmoke) (Variables|Default|GetisFogActive))
    (Niagara|SetNiagaraVariable(Vector3) (Variables|Default|GetNS_StylizedSmoke) "BoxSize" (Math|Vector|MakeVector (* (.x _tracehalfsize) 2.0) (* (.y _tracehalfsize) 2.0) (Math|Float|Lerp (.z (Transformation|GetWorldLocation (Variables|Default|GetScene))) (Variables|Default|GetmaxHeight) (/ _output_get _maxmovetimer))))
    (Variables|Default|SetCurrentHeight (Math|Float|Lerp (.z (Transformation|GetWorldLocation (Variables|Default|GetScene))) (Variables|Default|GetmaxHeight) (/ _output_get _maxmovetimer)))
    (bind _outhit (Collision|BoxTraceByChannel "0, 0, 0" (Math|Vector|MakeVector 0.0 0.0 (Math|Float|Lerp (.z (Transformation|GetWorldLocation (Variables|Default|GetScene))) (Variables|Default|GetmaxHeight) (/ _output_get _maxmovetimer))) (Variables|Default|GettraceHalfSize) "0, 0, 0" "TraceTypeQuery1" false 0 "ForOneFrame"))
    (bind _returnvalue (Actor|GetActorOfClass "/Game/Blueprint/Player/BP_CharacterPawn.BP_CharacterPawn_C"))
    (if (== _returnvalue (.hitactor _outhit))
      (Development|PrintString "CACA"))))